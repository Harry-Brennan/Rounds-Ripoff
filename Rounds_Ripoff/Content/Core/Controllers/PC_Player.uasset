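; PC_Player is the player controller for matches, handling UI screens, input state and camera hookup for BP_Player pawns.
; Owning-client events show and fade the waiting screen, play the map intro with input disabled, then re-enable input with Enhanced Input.
; The camera reference comes from the in-game player state; a multicast pushes colour and health info to pawns by index.
; Debug keys trigger player spawning and map intros through GM_Active_Game on the server.
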(event Custom|%28multi%29%20Update%20All%20Players%20Info
  (params (Colour :type Linear%20Color%20Structure) (Player :type Integer))
  (bind _outactors (Actor|GetAllActorsOfClass "/Game/Player/BP_Player.BP_Player_C"))
  (Class|BPIPlayer|SetupPlayer(Message) (Utilities|Array|Get(acopy) _outactors Player) (Utilities|Struct|MakeStruct_Player_Info Colour "NewEnumerator0" 1e+02)))

(event Custom|Enable%20In-Game%20Controls
  (Input|SetInputModeGameandUI self 0 "LockOnCapture" false false)
  (Variables|Default|SetbShowMouseCursor true)
  (Variables|Default|SetbEnableClickEvents true)
  (bind _asbp_player_state_in__game (Utilities|Casting|CastToBP_Player_State_In-Game (Variables|GetPlayerState)))
  (bind _camera_ref (Default|GetCameraRef _asbp_player_state_in__game))
  (bind _asbp_player (Utilities|Casting|CastToBP_Player (Pawn|GetControlledPawn)))
  (Default|SetupCameraRef _asbp_player _camera_ref))

(event Custom|%28owning%29%20Add%20Waiting%20Screen
  (bind _returnvalue (UserInterface|CreateWidget "/Game/UI/In_Game/WBP_Waiting_Screen.WBP_Waiting_Screen_C" self))
  (bind _output_get (Variables|Default|SetWaiting%20Screen%20Ref _returnvalue))
  (UserInterface|Viewport|AddtoViewport _output_get 0))

(event Custom|%28owning%29%20Fade%20Waiting%20Screen
  (bind _waiting_screen_ref (Variables|Default|GetWaiting%20Screen%20Ref))
  (Utilities|IsValid _waiting_screen_ref
    (:Is%20Valid
      (Default|FadeWaitingScreen _waiting_screen_ref)
      (bind _asbp_player_state_in__game (Utilities|Casting|CastToBP_Player_State_In-Game (Variables|GetPlayerState)))
      (bind _camera_ref (Default|GetCameraRef _asbp_player_state_in__game))
      (bind _asbp_player (Utilities|Casting|CastToBP_Player (Pawn|GetControlledPawn)))
      (Variables|/Game/Player/BP_Player.BP_Player_C|SetCamera%20Ref _asbp_player _camera_ref)
      (Variables|/Game/Player/BP_Player.BP_Player_C|SetLook%20At%20Cursor _asbp_player true))))

(event Custom|%28owning%29%20Enable%20Player%20Input
  (bind _self self)
  (bind _returnvalue (PlayerController|LocalPlayerSubsystems|GetEnhancedInputLocalPlayerSubsystem _self))
  (Utilities|IsValid (Pawn|GetControlledPawn)
    (:Is%20Valid
      (Input|EnableInput (Pawn|GetControlledPawn) self))
    (:Is%20Not%20Valid
      _))
  (Utilities|IsValid _returnvalue
    (:Is%20Valid
      (Input|AddMappingContext _returnvalue "/Game/Input/IMC_In-Game.IMC_In-Game" 0 "(bIgnoreAllPressedKeysUntilRelease=True,bForceImmediately=False,bNotifyUserSettings=False)"))))

(event Custom|%28owning%29%20Map%20Intro
  (params (Map%20Name :type String))
  (Utilities|IsValid (Pawn|GetControlledPawn)
    (:Is%20Valid
      (Input|DisableInput (Pawn|GetControlledPawn) self))
    (:Is%20Not%20Valid
      _))
  (bind _returnvalue (UserInterface|CreateWidget "/Game/UI/In_Game/WBP_Map_Intro.WBP_Map_Intro_C" self Map%20Name))
  (UserInterface|Viewport|AddtoViewport _returnvalue 0))

(event Custom|%28server%29%20Debug%20New%20Map
  (bind _asgm_active_game (Utilities|Casting|CastToGM_Active_Game (Game|GetGameMode)))
  (Default|MapIntro _asgm_active_game))

(event Input|KeyboardEvents|DebugKey9
  (params (Key :type Key%20Structure :default "None") (ActionValue :type Input%20Action%20Value%20Structure))
  (:Pressed
    (if (Pawn|IsLocalPlayerController)
      (Networking|SwitchHasAuthority
        (:Authority
          (bind _asgm_active_game (Utilities|Casting|CastToGM_Active_Game (Game|GetGameMode)))
          (Default|SpawnAllPlayers _asgm_active_game))))))

(event Input|KeyboardEvents|DebugKey0
  (params (Key :type Key%20Structure :default "None") (ActionValue :type Input%20Action%20Value%20Structure))
  (:Pressed
    (CallFunction|(server)DebugNewMap)))

(fn ConstructionScript)