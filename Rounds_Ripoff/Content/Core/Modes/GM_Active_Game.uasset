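; Game mode for a multiplayer elimination match, running players through rounds, maps and upgrade picks.
; It starts once all expected players log in, spawning them at random PlayerStarts tagged with the map name.
; Last-survivor checks score rounds; two wins take a map, then losers pick upgrades before another random map.
; UI updates fan out through PC_Player owning events; the game-over check reads just-reset round scores.
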(event Custom|Map%20Intro
  (for _array_element (Variables|Default|GetAll%20PCs)
    (bind _aspc_player (Utilities|Casting|CastToPC_Player _array_element))
    (Default|(owning)MapIntro _aspc_player (Variables|Map|GetCurrent%20Map%20Name))))

(event Custom|Add%20Upgrades%20Screen
  (params (Current%20Selecting%20Controller :type PC%20Player%20Object%20Reference))
  (for _array_element (Variables|Default|GetAll%20PCs)
    (bind _aspc_player (Utilities|Casting|CastToPC_Player _array_element))
    (Default|(owning)AddUpgradesScreen _aspc_player (== Current%20Selecting%20Controller _aspc_player) (Utilities|GetDisplayName Current%20Selecting%20Controller))))

(event Custom|Reset%20All%20Round%20Win%20Widgets%20Except%20Passed%20Index
  (params (Player%20Index :type Integer))
  (for _array_element (Variables|Default|GetAll%20PCs)
    (bind _aspc_player (Utilities|Casting|CastToPC_Player _array_element))
    (Default|(owning)ResetAllRoundWinsExceptPassed _aspc_player Player%20Index)))

(event Custom|Spawn%20All%20Players
  (bind _asbp_instance (Utilities|Casting|CastToBP_Instance (Game|GetGameInstance)))
  (for (_array_element _array_index) (Variables|Default|GetAll%20PCs)
    (Utilities|IsValid _array_element
      (:Is%20Valid
        (bind _aspc_player (Utilities|Casting|CastToPC_Player _array_element))
        (Spawning|SpawnPlayer _aspc_player (Utilities|Struct|MakeStruct_Player_Info (Utilities|Array|Get(acopy) (Variables|/Game/Core/Instances/BP_Instance.BP_Instance_C|GetPlayer%20Colours _asbp_instance) _array_index) "NewEnumerator0" 1e+02)))
      (:Is%20Not%20Valid
        (Development|PrintString "CONTROLLER NOT VALID WHEN SPAWNING ALL PLAYERS"))))
  (for _array_element_2 (Variables|Default|GetAll%20PCs)
    (bind _aspc_player_2 (Utilities|Casting|CastToPC_Player _array_element_2))
    (bind _asbp_player_state_in__game (Utilities|Casting|CastToBP_Player_State_In-Game (Variables|/Script/Engine.Controller|GetPlayerState _aspc_player_2)))
    (Default|UpdateCameraforController _asbp_player_state_in__game _aspc_player_2 (Variables|Map|GetCurrent%20Map%20Name))
    (Default|(owning)FadeWaitingScreen _aspc_player_2)))

(event Custom|Start%20Game
  (Utilities|FlowControl|Delay 2.0)
  (Development|PrintString (Utilities|String|Append (Utilities|String|ToString(Float) (Utilities|Time|GetGameTimeinSeconds)) " START GAME") true true "(R=0.000000,G=0.660000,B=1.000000,A=1.000000)" 1e+01)
  (CallFunction|SetupRoundandMapWins)
  (Round|StartRound))

(event Custom|Uncover%20Upgrade
  (params (Upgrade%20Index :type Integer))
  (for _array_element (Variables|Default|GetAll%20PCs)
    (bind _aspc_player (Utilities|Casting|CastToPC_Player _array_element))
    (Default|(owning)UncoverUpgrade _aspc_player Upgrade%20Index)))

(event Custom|Hover%20Upgrade
  (params (Upgrade%20Index :type Integer))
  (for _array_element (Variables|Default|GetAll%20PCs)
    (bind _aspc_player (Utilities|Casting|CastToPC_Player _array_element))
    (Default|(owning)HoverUpgrade _aspc_player Upgrade%20Index)))

(event Custom|Unhover%20Upgrade
  (params (Upgrade%20Index :type Integer))
  (for _array_element (Variables|Default|GetAll%20PCs)
    (bind _aspc_player (Utilities|Casting|CastToPC_Player _array_element))
    (Default|(owning)UnhoverUpgrade _aspc_player Upgrade%20Index)))

(event Custom|Pick%20Upgrade%20Anim
  (params (Upgrade%20Index :type Integer))
  (for _array_element (Variables|Default|GetAll%20PCs)
    (bind _aspc_player (Utilities|Casting|CastToPC_Player _array_element))
    (Default|(owning)PickUpgradeAnim _aspc_player Upgrade%20Index)))

(event Custom|Setup%20Map%20Win%20Display
  (bind _asbp_instance (Utilities|Casting|CastToBP_Instance (Game|GetGameInstance)))
  (for _array_element (Variables|Default|GetAll%20PCs)
    (bind _aspc_player (Utilities|Casting|CastToPC_Player _array_element))
    (Default|(owning)SetupMapWinDisplay _aspc_player (Utilities|Array|Length (Variables|Default|GetAll%20PCs)) (Variables|/Game/Core/Instances/BP_Instance.BP_Instance_C|GetPlayer%20Colours _asbp_instance))))

(event Custom|Add%20Round%20Win%20To%20Map%20Display
  (params (Player%20Index :type Integer))
  (for _array_element (Variables|Default|GetAll%20PCs)
    (bind _aspc_player (Utilities|Casting|CastToPC_Player _array_element))
    (Default|(owning)AddRoundWintoDisplay _aspc_player Player%20Index)))

(event EventPostLogin
  (params (NewPlayer :type Player%20Controller%20Object%20Reference))
  ;[0 0 0] Logged in
  (Utilities|Array|Add (Variables|Default|GetAll%20PCs) NewPlayer)
  (Development|PrintString (Utilities|String|Append (Utilities|String|ToString(Float) (Utilities|Time|GetGameTimeinSeconds)) " " (Utilities|GetDisplayName NewPlayer)) true true "(R=0.000000,G=0.155791,B=1.000000,A=1.000000)" 1e+02)
  (Utilities|FlowControl|Sequence
    (:then_0
      (bind _asbp_instance (Utilities|Casting|CastToBP_Instance (Game|GetGameInstance)))
      (if (and (== (Utilities|Array|LastIndex (Variables|Default|GetAll%20PCs)) (Utilities|Array|LastIndex (Variables|/Game/Core/Instances/BP_Instance.BP_Instance_C|GetPlayer%20Colours _asbp_instance))) (Class|GameStateBase|HasBegunPlay (Game|GetGameState)))
        (CallFunction|StartGame)))
    (:then_1
      (bind _aspc_player (Utilities|Casting|CastToPC_Player NewPlayer))
      (Default|(owning)AddWaitingScreen _aspc_player))))

(event EventOnLogout
  (params (ExitingController :type Controller%20Object%20Reference))
  ;[0 0 0] Logs out
  (bind _aspc_player (Utilities|Casting|CastToPC_Player ExitingController))
  (bind _asbp_instance (Utilities|Casting|CastToBP_Instance (Game|GetGameInstance)))
  (Default|RemovePlayerColour _asbp_instance (Utilities|Array|FindItem (Variables|Default|GetAll%20PCs) _aspc_player))
  (Utilities|Array|RemoveItem (Variables|Default|GetAll%20PCs) _aspc_player))

(event EventOnSwapPlayerControllers
  (params (OldPC :type Player%20Controller%20Object%20Reference) (NewPC :type Player%20Controller%20Object%20Reference))
  ;[0 0 0] Moving between levels but already logged in
  (Utilities|Array|Add (Variables|Default|GetAll%20PCs) NewPC)
  (Development|PrintString (Utilities|GetDisplayName NewPC) true true "(R=1.000000,G=0.019387,B=0.000000,A=1.000000)" 1e+02))

(fn ConstructionScript)

(fn FindRandomPlayerStart
  (LocalVariables|SetRandom%20Player%20Start (.OutItem (Utilities|Array|Random (Variables|Default|GetAvailable%20Player%20Spawns))))
  (Utilities|Array|RemoveItem (Variables|Default|GetAvailable%20Player%20Spawns) (LocalVariables|GetRandom%20Player%20Start))
  (return (Transformation|GetActorTransform (LocalVariables|GetRandom%20Player%20Start))))

(fn SpawnPlayer
  (params (Controller :type Player%20Controller%20Object%20Reference) (Player%20Info :type Struct%20Player%20Info%20Structure))
  (bind _returnvalue (Pawn|GetControlledPawn Controller))
  (Utilities|IsValid _returnvalue
    (:Is%20Valid
      (Actor|DestroyActor _returnvalue))
    (:Is%20Not%20Valid
      _))
  (bind _random_start_transform (Spawning|FindRandomPlayerStart))
  (bind _returnvalue_2 (Game|SpawnActorfromClass "/Game/Player/BP_Player.BP_Player_C" _random_start_transform "Undefined" "MultiplyWithRoot" 0 Player%20Info 0))
  (Pawn|Possess Controller _returnvalue_2))

(fn CheckRoundOver
  (Development|PrintString "CHECK ROUND OVER" true true "(R=0.000000,G=0.660000,B=1.000000,A=1.000000)" 1e+02)
  (bind _outactors (Actor|GetAllActorsOfClass "/Game/Player/BP_Player.BP_Player_C"))
  (for (_array_element _array_index) _outactors
    (if (<= (Variables|/Game/Health/BPC_Health.BPC_Health_C|GetCurrent%20Health (Actor|GetComponentbyClass _array_element "/Game/Health/BPC_Health.BPC_Health_C")) 0.0)
      (Math|Integer|IncrementInt (LocalVariables|GetPlayers%20Dead))
      (else
        (LocalVariables|SetRound%20Winner%20Index _array_index))))
  (if (<= (- (Utilities|Array|Length (Variables|Default|GetAll%20PCs)) (LocalVariables|GetPlayers%20Dead)) 1)
    (Round|RoundOver (LocalVariables|GetRound%20Winner%20Index))))

(fn RoundOver
  (params (Round%20Winner%20Index :type Integer))
  (Development|PrintString "ROUND OVER" true true "(R=0.000000,G=0.660000,B=1.000000,A=1.000000)" 1e+02)
  (Utilities|Array|SetArrayElem (Variables|Scores|GetPlayer%20Round%20Scores) Round%20Winner%20Index (+ (Utilities|Array|Get(acopy) (Variables|Scores|GetPlayer%20Round%20Scores) Round%20Winner%20Index) 1))
  (CallFunction|AddRoundWintoMapDisplay Round%20Winner%20Index)
  (Utilities|Time|SetTimerbyFunctionName 0 "Check Map Over" 2.0))

(fn CheckMapOver
  (Development|PrintString "CHECK MAP OVER" true true "(R=0.000000,G=0.660000,B=1.000000,A=1.000000)" 1e+02)
  (LocalVariables|SetMap%20Won? false)
  (bind (_array_element _array_index) (Utilities|Array|ForEachLoopwithBreak (Variables|Scores|GetPlayer%20Round%20Scores) :!label _label)
    (:LoopBody
      (Development|PrintString (Utilities|String|ToString(Integer) _array_element) true true "(R=1.000000,G=0.000000,B=0.068094,A=1.000000)" 1e+02)
      (if (>= _array_element 2)
        (LocalVariables|SetMap%20Won? true)
        (LocalVariables|SetMap%20Winner%20Index _array_index)
        (goto _label Break)))
    (:Completed
      (if (LocalVariables|GetMap%20Won?)
        (Variables|Map|SetCurrent%20Map%20Winner (LocalVariables|GetMap%20Winner%20Index))
        (Map|MapOver (LocalVariables|GetMap%20Winner%20Index))
        (else
          (Round|StartRound))))))

(fn MapOver
  (params (Map%20Winner%20Index :type Integer))
  (Development|PrintString "MAP OVER" true true "(R=0.000000,G=0.660000,B=1.000000,A=1.000000)" 1e+02)
  (Utilities|Array|SetArrayElem (Variables|Scores|GetPlayer%20Map%20Scores) Map%20Winner%20Index (+ (Utilities|Array|Get(acopy) (Variables|Scores|GetPlayer%20Map%20Scores) Map%20Winner%20Index) 1))
  (for (_ _array_index) (Variables|Scores|GetPlayer%20Round%20Scores)
    (Utilities|Array|SetArrayElem (Variables|Scores|GetPlayer%20Round%20Scores) _array_index 0))
  (CallFunction|ResetAllRoundWinWidgetsExceptPassedIndex Map%20Winner%20Index)
  (GameOver|CheckGameOver))

(fn CheckGameOver
  (Development|PrintString "CHECK GAME OVER")
  (LocalVariables|SetGame%20Won? false)
  (bind (_array_element _array_index) (Utilities|Array|ForEachLoopwithBreak (Variables|Scores|GetPlayer%20Round%20Scores) :!label _label)
    (:LoopBody
      (if (>= _array_element 5)
        (LocalVariables|SetGame%20Won? true)
        (LocalVariables|SetGame%20Winner%20Index _array_index)
        (goto _label Break)))
    (:Completed
      (if (LocalVariables|GetGame%20Won?)
        (GameOver|GameOver (LocalVariables|GetGame%20Winner%20Index))
        (else
          (Map|NextMap))))))

(fn GameOver
  (params (Game%20Winner%20Index :type Integer))
  (Development|PrintString (Utilities|String|Append "GAME OVER WINNER INDEX : " (Utilities|String|ToString(Integer) Game%20Winner%20Index))))

(fn NextMap
  (Map|RandomiseMap)
  (bind _outactors (Actor|GetAllActorsOfClasswithTag "/Script/Engine.PlayerStart" (Utilities|String|StringToName (Variables|Map|GetCurrent%20Map%20Name))))
  (Variables|Default|SetAvailable%20Player%20Spawns _outactors)
  (Utilities|Array|Clear (Variables|Map|GetUpgrade%20Indexes))
  (bind _aspc_player (Utilities|Casting|CastToPC_Player (Utilities|Array|Get(acopy) (Variables|Default|GetAll%20PCs) (Math|Integer|SelectInt 1 0 (== (Variables|Map|GetCurrent%20Map%20Winner) 0)))))
  (CallFunction|AddUpgradesScreen _aspc_player))

(fn MoveSpawnedPlayers
  (bind _outactors (Actor|GetAllActorsOfClasswithTag "/Script/Engine.PlayerStart" (Utilities|String|StringToName (Variables|Map|GetCurrent%20Map%20Name))))
  (Variables|Default|SetAvailable%20Player%20Spawns _outactors)
  (for _array_element (Variables|Default|GetAll%20PCs)
    (bind _random_start_transform (Spawning|FindRandomPlayerStart))
    (Transformation|SetActorTransform (Pawn|GetControlledPawn _array_element) _random_start_transform)))

(fn RandomiseMap
  (bind _returnvalue (|GetNumEnumEntries))
  (bind _returnvalue_2 (- _returnvalue 1))
  (bind _returnvalue_3 (Math|Random|RandomIntegerinRange 0 _returnvalue_2))
  (bind _returnvalue_4 (Math|Conversions|ToByte(Integer) _returnvalue_3))
  (bind _returnvalue_5 (Utilities|Enum|ByteToEnumEnum_Map_Names _returnvalue_4))
  (bind _returnvalue_6 (Utilities|String|EnumtoString _returnvalue_5))
  (Variables|Map|SetPrevious%20Map%20Name (Variables|Map|GetCurrent%20Map%20Name))
  (LocalVariables|SetPotential%20New%20Map%20Name _returnvalue_6)
  (if (Utilities|Enum|Equal(Enum) _returnvalue_6 (Variables|Map|GetPrevious%20Map%20Name))
    (Map|RandomiseMap)
    (else
      (bind _output_get (Variables|Map|SetCurrent%20Map%20Name (LocalVariables|GetPotential%20New%20Map%20Name))))))

(fn StartRound
  (Development|PrintString "START ROUND")
  (for _array_element (Variables|Default|GetAll%20PCs)
    (bind _aspc_player (Utilities|Casting|CastToPC_Player _array_element))
    (Default|ResetAllPlayers _aspc_player))
  (Utilities|IsValid (Pawn|GetControlledPawn (Utilities|Array|Get(acopy) (Variables|Default|GetAll%20PCs)))
    (:Is%20Valid
      (Round|MoveSpawnedPlayers)
      (for _array_element_2 (Variables|Default|GetAll%20PCs)
        (bind _aspc_player_2 (Utilities|Casting|CastToPC_Player _array_element_2))
        (bind _asbp_player_state_in__game (Utilities|Casting|CastToBP_Player_State_In-Game (Variables|/Script/Engine.Controller|GetPlayerState _aspc_player_2)))
        (Default|UpdateCameraforController _asbp_player_state_in__game _aspc_player_2 (Variables|Map|GetCurrent%20Map%20Name)))
      (CallFunction|MapIntro))
    (:Is%20Not%20Valid
      (Variables|Map|SetCurrent%20Map%20Name (Utilities|String|EnumtoString (Utilities|Enum|ByteToEnumEnum_Map_Names (Math|Conversions|ToByte(Integer) (Math|Random|RandomIntegerinRange 0 (- (|GetNumEnumEntries) 1))))))
      (bind _outactors (Actor|GetAllActorsOfClasswithTag "/Script/Engine.PlayerStart" (Utilities|String|StringToName (Variables|Map|GetCurrent%20Map%20Name))))
      (Variables|Default|SetAvailable%20Player%20Spawns _outactors)
      (CallFunction|SpawnAllPlayers))))

(fn SetupRoundandMapWins
  (for _array_element (Variables|Default|GetAll%20PCs)
    (Utilities|Array|Add (Variables|Scores|GetPlayer%20Round%20Scores) 0)
    (Utilities|Array|Add (Variables|Scores|GetPlayer%20Map%20Scores) 0))
  (CallFunction|SetupMapWinDisplay))

(fn UpgradeAdded
  (params (Upgrade :type Enum_Upgrades%20Enum :default "NewEnumerator0") (Controller :type PC%20Player%20Object%20Reference))
  (bind _all_pcs (Variables|Default|GetAll%20PCs))
  (bind _returnvalue (Utilities|Array|FindItem _all_pcs Controller))
  (bind _returnvalue_2 (+ _returnvalue 1))
  (for _array_element (Variables|Default|GetAll%20PCs)
    (bind _aspc_player (Utilities|Casting|CastToPC_Player _array_element))
    (Default|(owning)RemoveUpgradesScreen _aspc_player))
  (Default|AddUpgradetoPlayer Controller Upgrade)
  (Utilities|Array|Add (Variables|Map|GetUpgrade%20Indexes) 0)
  (if (== (Utilities|Array|Length (Variables|Map|GetUpgrade%20Indexes)) (- (Utilities|Array|Length (Variables|Default|GetAll%20PCs)) 1))
    (Round|StartRound)
    (else
      (bind _aspc_player_2 (Utilities|Casting|CastToPC_Player (Utilities|Array|Get(acopy) _all_pcs (Math|Integer|SelectInt (+ _returnvalue_2 1) _returnvalue_2 (== (Variables|Map|GetCurrent%20Map%20Winner) _returnvalue_2)))))
      (CallFunction|AddUpgradesScreen _aspc_player_2))))