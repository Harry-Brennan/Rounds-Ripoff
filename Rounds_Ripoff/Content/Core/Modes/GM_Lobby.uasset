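; Lobby game mode that tracks joining and leaving PC_Lobby controllers, their ready states and player colour claims, refreshing lobby info through server calls.
; When all are ready it starts a countdown and timer, cancelling both if anyone unreadies.
; On expiry it shows loading screens, server-travels to ThirdPersonMap and copies used colours to BP_Instance.
; GetAvailableColour cycles forward or backward through unused colours, wrapping around.
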(event Custom|Remove%20Available%20Colour
  (params (Colour :type Linear%20Color%20Structure))
  (if (not (== Colour "(R=0.000000,G=0.000000,B=0.000000,A=0.000000)"))
    (Utilities|Map|Add (Variables|Default|GetPossible%20Player%20Colours%20-%20Used) Colour true)))

(event Custom|Add%20Available%20Colour
  (params (Colour :type Linear%20Color%20Structure))
  (if (not (== Colour "(R=0.000000,G=0.000000,B=0.000000,A=0.000000)"))
    (Utilities|Map|Add (Variables|Default|GetPossible%20Player%20Colours%20-%20Used) Colour false)))

(event Custom|Update%20Player%20Ready
  (params (Ready? :type Boolean) (Controller :type PC%20Lobby%20Object%20Reference))
  (Utilities|Array|SetArrayElem (Variables|Default|GetPlayer%20Ready%20States) (Utilities|Array|FindItem (Variables|Default|GetAll%20PCs) Controller) Ready?)
  (Variables|Default|SetAll%20Players%20Ready? true)
  (for _array_element (Variables|Default|GetPlayer%20Ready%20States)
    (if (not _array_element)
      (Variables|Default|SetAll%20Players%20Ready? false)))
  (if (Variables|Default|GetAll%20Players%20Ready?)
    (Utilities|Time|ClearandInvalidateTimerbyHandle (Variables|Default|GetStart%20Game%20Timer))
    (for _array_element_2 (Variables|Default|GetAll%20PCs)
      (Default|(owning)StartCountdown _array_element_2))
    (bind _returnvalue (Utilities|Time|SetTimerbyEvent (delegate Custom|Start%20Game) 5.0))
    (Variables|Default|SetStart%20Game%20Timer _returnvalue)
    (else
      (Utilities|Time|ClearandInvalidateTimerbyHandle (Variables|Default|GetStart%20Game%20Timer))
      (for _array_element_3 (Variables|Default|GetAll%20PCs)
        (Default|(owning)StopCountdown _array_element_3)))))

(event Custom|Start%20Game
  (bind _possible_player_colours___used (Variables|Default|GetPossible%20Player%20Colours%20-%20Used))
  (Development|PrintString "START GAME")
  (for _array_element (Variables|Default|GetAll%20PCs)
    (Default|(owning)StopCountdown _array_element))
  (for _array_element_2 (Variables|Default|GetAll%20PCs)
    (Default|(owning)LoadingScreenIntoLevel _array_element_2))
  (Development|ExecuteConsoleCommand "servertravel ThirdPersonMap" 0)
  (bind _asbp_instance (Utilities|Casting|CastToBP_Instance (Game|GetGameInstance)))
  (Utilities|Array|Clear (Variables|/Game/Core/Instances/BP_Instance.BP_Instance_C|GetPlayer%20Colours _asbp_instance))
  (bind _keys (Utilities|Map|Keys _possible_player_colours___used))
  (for _array_element_3 _keys
    (if (.Value (Utilities|Map|Find _possible_player_colours___used _array_element_3))
      (Utilities|Array|Add (Variables|/Game/Core/Instances/BP_Instance.BP_Instance_C|GetPlayer%20Colours _asbp_instance) _array_element_3))))

(event EventTick
  (params (DeltaSeconds :type Float%20%28single-precision%29))
  (if (> (Utilities|Array|Length (Variables|Default|GetAll%20PCs)) 1)
    (for _array_element (Variables|Default|GetAll%20PCs)
      (Default|(server)UpdateLobbyPlayerInfo _array_element))))

(event EventPostLogin
  (params (NewPlayer :type Player%20Controller%20Object%20Reference))
  ;[0 0 0] Logged in
  (bind _aspc_lobby (Utilities|Casting|CastToPC_Lobby NewPlayer))
  (Utilities|Array|Add (Variables|Default|GetAll%20PCs) _aspc_lobby)
  (Utilities|Array|Add (Variables|Default|GetPlayer%20Ready%20States) false)
  (for _array_element (Variables|Default|GetAll%20PCs)
    (if (Pawn|IsLocalController _array_element)
      (Default|(server)UpdateLobbyPlayerInfo _array_element))))

(event EventOnLogout
  (params (ExitingController :type Controller%20Object%20Reference))
  (bind _all_pcs (Variables|Default|GetAll%20PCs))
  (bind _output (Utilities|Array|Get(acopy) _all_pcs))
  ;[0 0 0] Logs out
  (bind _aspc_lobby (Utilities|Casting|CastToPC_Lobby ExitingController))
  (Utilities|Array|RemoveIndex (Variables|Default|GetPlayer%20Ready%20States) (Utilities|Array|FindItem (Variables|Default|GetAll%20PCs) _aspc_lobby))
  (Utilities|IsValid _output
    (:Is%20Valid
      (Default|(server)RemovePlayerInfo _output _aspc_lobby))
    (:Is%20Not%20Valid
      _))
  (Utilities|Array|RemoveItem (Variables|Default|GetAll%20PCs) _aspc_lobby))

(event EventOnSwapPlayerControllers
  (params (OldPC :type Player%20Controller%20Object%20Reference) (NewPC :type Player%20Controller%20Object%20Reference))
  ;[0 0 0] Moving between levels but already logged in
  (bind _aspc_lobby (Utilities|Casting|CastToPC_Lobby NewPC))
  (Utilities|Array|Add (Variables|Default|GetAll%20PCs) _aspc_lobby)
  (Utilities|Array|Add (Variables|Default|GetPlayer%20Ready%20States) false)
  (for _array_element (Variables|Default|GetAll%20PCs)
    (if (Pawn|IsLocalController _array_element)
      (Default|(server)UpdateLobbyPlayerInfo _array_element))))

(fn ConstructionScript)

(fn GetAvailableColour
  (params (Next :type Boolean) (Current%20Colour :type Linear%20Color%20Structure))
  (bind _keys (Utilities|Map|Keys (Variables|Default|GetPossible%20Player%20Colours%20-%20Used)))
  (bind _output_get (LocalVariables|SetInverted%20Order%20Player%20Colours _keys))
  (Utilities|Array|Reverse _output_get)
  (LocalVariables|SetCurrent%20Colour%20Index (Math|Integer|SelectInt (Utilities|Array|FindItem _keys Current%20Colour) (Utilities|Array|FindItem (LocalVariables|GetInverted%20Order%20Player%20Colours) Current%20Colour) Next))
  (if Next
    (bind (_array_element _array_index) (Utilities|Array|ForEachLoopwithBreak _keys :!label _label)
      (:LoopBody
        (if (and (not (.Value (Utilities|Map|Find (Variables|Default|GetPossible%20Player%20Colours%20-%20Used) _array_element))) (> _array_index (LocalVariables|GetCurrent%20Colour%20Index)))
          (LocalVariables|SetFound%20Colour true)
          (LocalVariables|SetNext%20Colour _array_element)
          (goto _label Break)))
      (:Completed
        (if (LocalVariables|GetFound%20Colour) :!label _label_2
          (return (LocalVariables|GetNext%20Colour))
          (else
            (bind _array_element_2 (Utilities|Array|ForEachLoopwithBreak (select Next _keys (LocalVariables|GetInverted%20Order%20Player%20Colours)) :!label _label_3)
              (:LoopBody
                (if (not (.Value (Utilities|Map|Find (Variables|Default|GetPossible%20Player%20Colours%20-%20Used) _array_element_2)))
                  (LocalVariables|SetFound%20Colour true)
                  (LocalVariables|SetNext%20Colour _array_element_2)
                  (goto _label_3 Break)))
              (:Completed
                (if (LocalVariables|GetFound%20Colour)
                  (return (LocalVariables|GetNext%20Colour))
                  (else
                    (return "(R=1.000000,G=1.000000,B=1.000000,A=0.000000)")))))))))
    (else
      (bind (_array_element_3 _array_index_2) (Utilities|Array|ForEachLoopwithBreak (LocalVariables|GetInverted%20Order%20Player%20Colours) :!label _label_4)
        (:LoopBody
          (if (and (not (.Value (Utilities|Map|Find (Variables|Default|GetPossible%20Player%20Colours%20-%20Used) _array_element_3))) (> _array_index_2 (LocalVariables|GetCurrent%20Colour%20Index)))
            (LocalVariables|SetFound%20Colour true)
            (LocalVariables|SetNext%20Colour _array_element_3)
            (goto _label_4 Break)))
        (:Completed
          (goto _label_2))))))