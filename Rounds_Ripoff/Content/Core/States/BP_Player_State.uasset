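; BP_Player_State sets up each player's pawn info and hands the local view to the level's shared BP_Camera.
; On BeginPlay it caches the camera actor, which it also exposes through a getter.
; A multicast UpdatePlayerInfo rolls random colour and max health on each machine, then sends them to the controlled pawn.
; For local controllers it then blends to the camera and enables cursor look-at once the blend time elapses.
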(event Custom|Update%20Camera%20For%20Player
  (params (Player :type BP%20Player%20Object%20Reference) (Controller :type Player%20Controller%20Object%20Reference))
  (if (Pawn|IsLocalController Controller)
    (Game|Player|SetViewTargetwithBlend Controller (Variables|Default|GetCamera%20Ref) 1.0 "VTBlend_Linear" 0.0 false)
    (Variables|/Game/Player/BP_Player.BP_Player_C|SetCamera%20Ref Player (Variables|Default|GetCamera%20Ref))
    (Utilities|FlowControl|Delay 1.0)
    (Variables|/Game/Player/BP_Player.BP_Player_C|SetLook%20At%20Cursor Player true)))

(event Custom|%28multi%29%20Update%20Player%20Info
  (params (Controller :type Player%20Controller%20Object%20Reference))
  (bind _returnvalue (Pawn|GetControlledPawn Controller))
  (bind _returnvalue_2 (Math|Random|RandomInteger 4))
  (Utilities|IsValid Controller
    (:Is%20Valid
      (Class|BPIPlayer|SetupPlayer(Message) _returnvalue (Utilities|Struct|MakeStruct_Player_Info (Utilities|Select :Index _returnvalue_2 :Option%200 "(R=1.000000,G=0.000000,B=0.207326,A=1.000000)" :Option%201 "(R=0.171296,G=0.000000,B=1.000000,A=1.000000)" :Option%202 "(R=0.000000,G=1.000000,B=0.498256,A=1.000000)" :Option%203 "(R=1.000000,G=0.944142,B=0.000000,A=1.000000)") "NewEnumerator0" (Utilities|Select :Index _returnvalue_2 :Option%200 2e+01 :Option%201 4e+01 :Option%202 6e+01 :Option%203 8e+01)))
      (bind _asbp_player (Utilities|Casting|CastToBP_Player _returnvalue))
      (CallFunction|UpdateCameraforPlayer _asbp_player Controller))))

(event EventBeginPlay
  (Development|PrintString (Utilities|GetDisplayName self) true true "(R=1.000000,G=0.000000,B=0.000000,A=1.000000)")
  (bind _returnvalue (Actor|GetActorOfClass "/Game/Player/Camera/BP_Camera.BP_Camera_C"))
  (Variables|Default|SetCamera%20Ref _returnvalue))

(fn ConstructionScript)

(fn GetCameraRef
  (return (Variables|Default|GetCamera%20Ref)))