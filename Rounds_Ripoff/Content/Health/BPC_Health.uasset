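; Health component that tracks its owner's current and maximum health, handling damage, healing and player death.
; Server events relay damage and healing to multicasts that adjust health on each machine, rather than visibly relying on replicated variables.
; Non-lethal hits trigger the owner's blood effect component.
; Lethal hits call server death, which for BPI_Player owners switches to UI-only input, multicasts a blood explosion, asks GM_Active_Game to check round over, and hides owner and weapon.
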(event Custom|%28server%29%20Take%20Damage
  (params (Damage :type Float%20%28double-precision%29) (Location%20Of%20Damage :type Vector))
  ;[0 0 0] Take Damage
  (CallFunction|(multi)TakeDamage Damage Location%20Of%20Damage))

(event Custom|%28server%29%20Death
  ;[0 0 0] Death
  (CallFunction|Death))

(event Custom|%28server%29%20Update%20Health%20Info
  (params (New%20Maximum :type Float%20%28double-precision%29))
  (CallFunction|UpdateHealthInfo New%20Maximum))

(event Custom|Update%20Health%20Info
  (params (New%20Maximum :type Float%20%28double-precision%29))
  (bind _output_get (Variables|Default|SetCurrent%20Health New%20Maximum))
  (Variables|Default|SetMaximum%20Health _output_get))

(event Custom|%28multi%29%20Take%20Damage
  (params (Damage :type Float%20%28double-precision%29) (Location%20of%20Damage :type Vector))
  ;[0 0 0] Take Damage
  (Development|PrintString (Utilities|String|Append (Utilities|GetDisplayName (Components|GetOwner)) " TAKE DAMAGE"))
  (if (<= (- (Variables|Default|GetCurrent%20Health) Damage) 0.0)
    (Variables|Default|SetCurrent%20Health (- (Variables|Default|GetCurrent%20Health) Damage))
    (CallFunction|(server)Death)
    (else
      (Variables|Default|SetCurrent%20Health (- (Variables|Default|GetCurrent%20Health) Damage))
      (CallFunction|(server)TakeDamageCosmetic Location%20of%20Damage))))

(event Custom|Death
  ;[0 0 0] Death
  ;[0 0 0] Player Specific Death
  (if (Utilities|DoesObjectImplementInterface (Components|GetOwner) "/Game/Player/BPI_Player.BPI_Player_C")
    (bind _controller (Class|BPIPlayer|GetPlayer'sController(Message) (Components|GetOwner)))
    (Input|SetInputModeUIOnly _controller 0 "DoNotLock" false)
    (CallFunction|(server)DeathCosmetic)
    (bind _asgm_active_game (Utilities|Casting|CastToGM_Active_Game (Game|GetGameMode)))
    (Default|CheckRoundOver _asgm_active_game)
    (Rendering|SetActorHiddenInGame (Variables|/Game/Combat/Weapons/BPC_Weaponry.BPC_Weaponry_C|GetWeapon%20Ref (Actor|GetComponentbyClass (Components|GetOwner) "/Game/Combat/Weapons/BPC_Weaponry.BPC_Weaponry_C")) true)))

(event Custom|%28server%29%20Heal
  (params (Heal :type Float%20%28double-precision%29))
  ;[0 0 0] Healing
  (CallFunction|(multi)Heal Heal))

(event Custom|%28multi%29%20Heal
  (params (Heal :type Float%20%28double-precision%29))
  ;[0 0 0] Healing
  (if (> (Variables|Default|GetCurrent%20Health) 0.0)
    (Variables|Default|SetCurrent%20Health (Math|Float|Clamp(Float) (+ (Variables|Default|GetCurrent%20Health) Heal) 0.0 (Variables|Default|GetMaximum%20Health)))))

(event Custom|%28server%29%20Death%20Cosmetic
  ;[0 0 0] Cosmetic Effects of death that should replicate to all players
  (CallFunction|(multi)DeathCosmetic))

(event Custom|%28multi%29%20Death%20Cosmetic
  ;[0 0 0] Cosmetic Effects of death that should replicate to all players
  (Game|SpawnActorfromClass "/Game/VFX/Bloodsplosion/BPs/BP_BloodSplosion.BP_BloodSplosion_C" (Math|Transform|MakeTransform (Transformation|GetActorLocation (Components|GetOwner)) "0, 0, 0" "1.000000,1.000000,1.000000") "Undefined" "MultiplyWithRoot" 0 500 0))

(event Custom|%28server%29%20Take%20Damage%20Cosmetic
  (params (Location%20Of%20Damage :type Vector))
  ;[0 0 0] Take Damage
  (CallFunction|(multi)TakeDamageCosmetic Location%20Of%20Damage))

(event Custom|%28multi%29%20Take%20Damage%20Cosmetic
  (params (Location%20Of%20Damage :type Vector))
  ;[0 0 0] Take Damage
  (Default|BloodEffect (Actor|GetComponentbyClass (Components|GetOwner) "/Game/VFX/Blood_Splatter/BPS/BPC_Blood_Effect.BPC_Blood_Effect_C") (Transformation|GetActorLocation (Components|GetOwner)) (- (Transformation|GetActorLocation (Components|GetOwner)) Location%20Of%20Damage) (Components|GetOwner) 2e+01))