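; Camera actor that, after a countdown, gradually zooms its spring arm and shrinks the surrounding walls toward a center point.
; A multicast start event resets zoom and walls, then sets the timer that plays a rate-scaled timeline.
; The timeline lerps arm length and slides each wall horizontally from its cached original position toward a minimum distance from the center, preserving height.
; Zoom and wall shrinking have separate toggles, with multicast resets.
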(event Custom|%28multi%29%20Start%20Countdown%20For%20Zoom%20Start
  (if (Variables|ZoomVariables|GetShould%20Zoomin?)
    (CallFunction|(multi)CameraZoomReset)
    (bind _returnvalue (Utilities|Time|SetTimerbyEvent (delegate Custom|Camera%20Zoom%20Start) (Variables|Countdown|GetCountdown%20Till%20Start%20Zooming)))
    (Variables|Countdown|SetZoom%20Countdown%20Timer _returnvalue)
    (if (Variables|ShrinkingWalls|GetShould%20Shrink%20Walls?)
      (CallFunction|(multi)WallsReset))))

(event Custom|Camera%20Zoom%20Start
  (Components|Timeline|SetPlayRate (Variables|Default|GetCamera%20Zoom%20Timeline) (/ 1.0 (Variables|ZoomVariables|GetCamera%20Zoom%20Time%20to%20Complete)))
  (bind _alpha (Timeline|Camera%20Zoom%20Timeline PlayFromStart)
    (:Update
      (Variables|/Script/Engine.SpringArmComponent|SetTargetArmLength (Variables|Default|GetSpringArm) (Math|Float|Lerp (Variables|ZoomVariables|GetDefault%20Zoom%20Amount) (Variables|ZoomVariables|GetFinal%20Zoom%20Amount) _alpha))
      (for (_array_element _array_index) (Variables|ShrinkingWalls|GetWalls%20To%20Shrink)
        (if (> (Math|Vector|Distance(Vector) (Transformation|GetWorldLocation (Variables|Default|GetCenter)) (Transformation|GetActorLocation _array_element)) (Variables|ShrinkingWalls|GetMin%20Wall%20Distance%20to%20Camera))
          (Transformation|SetActorLocation _array_element (Math|Vector|Lerp(Vector) (Utilities|Array|Get(acopy) (Variables|ShrinkingWalls|GetOriginal%20Wall%20Positions) _array_index) (Math|Vector|MakeVector (.x (+ (* (Math|Vector|GetForwardVector (Math|Rotator|FindLookatRotation (Transformation|GetWorldLocation (Variables|Default|GetCenter)) (Utilities|Array|Get(acopy) (Variables|ShrinkingWalls|GetOriginal%20Wall%20Positions) _array_index))) (Variables|ShrinkingWalls|GetMin%20Wall%20Distance%20to%20Camera)) (Transformation|GetWorldLocation (Variables|Default|GetCenter)))) (.y (+ (* (Math|Vector|GetForwardVector (Math|Rotator|FindLookatRotation (Transformation|GetWorldLocation (Variables|Default|GetCenter)) (Utilities|Array|Get(acopy) (Variables|ShrinkingWalls|GetOriginal%20Wall%20Positions) _array_index))) (Variables|ShrinkingWalls|GetMin%20Wall%20Distance%20to%20Camera)) (Transformation|GetWorldLocation (Variables|Default|GetCenter)))) (.Z (Math|Vector|BreakVector (Utilities|Array|Get(acopy) (Variables|ShrinkingWalls|GetOriginal%20Wall%20Positions) _array_index)))) _alpha) false false))))))

(event Custom|Camera%20Zoom%20Stop
  (bind _alpha (Timeline|Camera%20Zoom%20Timeline Stop)
    (:Update
      (Variables|/Script/Engine.SpringArmComponent|SetTargetArmLength (Variables|Default|GetSpringArm) (Math|Float|Lerp (Variables|ZoomVariables|GetDefault%20Zoom%20Amount) (Variables|ZoomVariables|GetFinal%20Zoom%20Amount) _alpha))
      (for (_array_element _array_index) (Variables|ShrinkingWalls|GetWalls%20To%20Shrink)
        (if (> (Math|Vector|Distance(Vector) (Transformation|GetWorldLocation (Variables|Default|GetCenter)) (Transformation|GetActorLocation _array_element)) (Variables|ShrinkingWalls|GetMin%20Wall%20Distance%20to%20Camera))
          (Transformation|SetActorLocation _array_element (Math|Vector|Lerp(Vector) (Utilities|Array|Get(acopy) (Variables|ShrinkingWalls|GetOriginal%20Wall%20Positions) _array_index) (Math|Vector|MakeVector (.x (+ (* (Math|Vector|GetForwardVector (Math|Rotator|FindLookatRotation (Transformation|GetWorldLocation (Variables|Default|GetCenter)) (Utilities|Array|Get(acopy) (Variables|ShrinkingWalls|GetOriginal%20Wall%20Positions) _array_index))) (Variables|ShrinkingWalls|GetMin%20Wall%20Distance%20to%20Camera)) (Transformation|GetWorldLocation (Variables|Default|GetCenter)))) (.y (+ (* (Math|Vector|GetForwardVector (Math|Rotator|FindLookatRotation (Transformation|GetWorldLocation (Variables|Default|GetCenter)) (Utilities|Array|Get(acopy) (Variables|ShrinkingWalls|GetOriginal%20Wall%20Positions) _array_index))) (Variables|ShrinkingWalls|GetMin%20Wall%20Distance%20to%20Camera)) (Transformation|GetWorldLocation (Variables|Default|GetCenter)))) (.Z (Math|Vector|BreakVector (Utilities|Array|Get(acopy) (Variables|ShrinkingWalls|GetOriginal%20Wall%20Positions) _array_index)))) _alpha) false false))))))

(event Custom|%28multi%29%20Camera%20Zoom%20Reset
  (CallFunction|CameraZoomStop)
  (Variables|/Script/Engine.SpringArmComponent|SetTargetArmLength (Variables|Default|GetSpringArm) (Variables|ZoomVariables|GetDefault%20Zoom%20Amount)))

(event Custom|Setup%20Camera%20Walls
  (if (Variables|ShrinkingWalls|GetShould%20Shrink%20Walls?)
    (for _array_element (Variables|ShrinkingWalls|GetWalls%20To%20Shrink)
      (Utilities|Array|Add (Variables|ShrinkingWalls|GetOriginal%20Wall%20Positions) (Transformation|GetActorLocation _array_element)))))

(event Custom|%28multi%29%20Walls%20Reset
  (for (_array_element _array_index) (Variables|ShrinkingWalls|GetWalls%20To%20Shrink)
    (Transformation|SetActorLocation _array_element (Utilities|Array|Get(acopy) (Variables|ShrinkingWalls|GetOriginal%20Wall%20Positions) _array_index) false false)))

(event EventBeginPlay
  (CallFunction|SetupCameraWalls))

(fn ConstructionScript)