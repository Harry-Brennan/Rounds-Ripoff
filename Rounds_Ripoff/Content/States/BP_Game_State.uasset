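; Game State that starts the match once every player reports ready.
; CheckAllPlayersReady queries each entry in PlayerArray through GetPlayerReadyMessage and sets GameCanStart only if all are ready.
; It then branches on authority, calling the StartGame multicast directly or through a server RPC.
; The multicast calls SetupPlayerMessage on each player's controlled pawn, with debug prints marking the server and multicast steps.
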(event Custom|%28server%29%20Start%20Game
  (CallFunction|(multi)StartGame)
  (Development|PrintString "SERVER START GAME"))

(event Custom|%28multi%29%20Start%20Game
  (Development|PrintString "MULTI START GAME")
  (for _array_element (Variables|Default|GetPlayerArray)
    (Class|BPIPlayer|SetupPlayer(Message) (Pawn|GetControlledPawn (Game|GetPlayerController _array_element)))))

(event EventCheckAllPlayersReady
  (Variables|Default|SetGame%20Can%20Start true)
  (for _array_element (Variables|Default|GetPlayerArray)
    (bind _ready (Class|BPIPlayerState|GetPlayerReady(Message) _array_element))
    (if (not _ready)
      (Variables|Default|SetGame%20Can%20Start false)))
  (if (Variables|Default|GetGame%20Can%20Start)
    (Networking|SwitchHasAuthority
      (:Authority
        (CallFunction|(multi)StartGame))
      (:Remote
        (CallFunction|(server)StartGame)))))

(fn ConstructionScript)