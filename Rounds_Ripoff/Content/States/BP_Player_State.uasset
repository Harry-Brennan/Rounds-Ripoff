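; Player state Blueprint that sets up the shared camera for players and tracks a player-ready flag.
; On BeginPlay it finds the BP_Camera, blends every BP_Player's controller view to it and passes them the reference, then enables cursor look-at after a delay.
; Ready changes branch on authority, going through a server RPC from clients and a multicast to set the flag everywhere.
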(event Custom|%28server%29%20Update%20Player%20Ready
  (params (Ready :type Boolean))
  (CallFunction|(multi)UpdatePlayerReady Ready))

(event Custom|%28multi%29%20Update%20Player%20Ready
  (params (Ready :type Boolean))
  (Variables|Default|SetPlayer%20Ready Ready))

(event EventBeginPlay
  (Development|PrintString (Utilities|GetDisplayName self) true true "(R=1.000000,G=0.000000,B=0.000000,A=1.000000)")
  (bind _returnvalue (Actor|GetActorOfClass "/Game/Player/Camera/BP_Camera.BP_Camera_C"))
  (Variables|Default|SetCamera%20Ref _returnvalue)
  (Utilities|FlowControl|Delay 0.2)
  (bind _outactors (Actor|GetAllActorsOfClass "/Game/Player/BP_Player.BP_Player_C"))
  (for _array_element _outactors
    (bind _asplayer_controller (Utilities|Casting|CastToPlayerController (Pawn|GetController _array_element)))
    (Game|Player|SetViewTargetwithBlend _asplayer_controller (Variables|Default|GetCamera%20Ref) 1.0 "VTBlend_Linear" 0.0 false)
    (Variables|/Game/Player/BP_Player.BP_Player_C|SetCamera%20Ref _array_element (Variables|Default|GetCamera%20Ref)))
  (Utilities|FlowControl|Delay 4.0)
  (bind _outactors_2 (Actor|GetAllActorsOfClass "/Game/Player/BP_Player.BP_Player_C"))
  (for _array_element_2 _outactors_2
    (Variables|/Game/Player/BP_Player.BP_Player_C|SetLook%20At%20Cursor _array_element_2 true)))

(event EventUpdatePlayerReady
  (params (Ready :type Boolean))
  (Networking|SwitchHasAuthority
    (:Authority
      (CallFunction|(multi)UpdatePlayerReady Ready))
    (:Remote
      (CallFunction|(server)UpdatePlayerReady Ready))))

(fn ConstructionScript)

(fn GetCameraRef
  (return (Variables|Default|GetCamera%20Ref)))

(fn GetPlayerReady
  (return (Variables|Default|GetPlayer%20Ready)))