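; Active-game mode Blueprint that hands out per-player colour and max health to every BP_Player.
; An interface event routes through a server event to the update, which loops over all BP_Player actors.
; Each actor's array index selects one of four preset colour and health pairs, sent in a PlayerInfo struct through the player's ServerUpdatePlayerInfo.
; Each assignment prints the actor name and index for debugging.
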(event Custom|%28server%29%20Update%20Player%20Info
  (CallFunction|UpdatePlayerInfo))

(event Custom|Update%20Player%20Info
  (bind _outactors (Actor|GetAllActorsOfClass "/Game/Player/BP_Player.BP_Player_C"))
  (for (_array_element _array_index) _outactors
    (Default|(server)UpdatePlayerInfo _array_element (Utilities|Struct|MakeStruct_Player_Info (Utilities|Select :Index _array_index :Option%200 "(R=1.000000,G=0.000000,B=0.207326,A=1.000000)" :Option%201 "(R=0.171296,G=0.000000,B=1.000000,A=1.000000)" :Option%202 "(R=0.000000,G=1.000000,B=0.498256,A=1.000000)" :Option%203 "(R=1.000000,G=0.944142,B=0.000000,A=1.000000)") "NewEnumerator0" (Utilities|Select :Index _array_index :Option%200 2e+01 :Option%201 4e+01 :Option%202 6e+01 :Option%203 8e+01)))
    (Development|PrintString (Utilities|String|Append (Utilities|GetDisplayName _array_element) " - " (Utilities|String|ToString(Integer) _array_index)))))

(event Event(interface)UpdatePlayerInfo
  (CallFunction|(server)UpdatePlayerInfo))

(fn ConstructionScript)