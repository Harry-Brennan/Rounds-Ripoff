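; Animation notify state that turns the owning character's weapon hitbox on for a marked window of an animation.
; On begin and end it finds the mesh owner's BPC_Weaponry component and calls ActivateHitbox or DeactivateHitbox on its WeaponRef.
; The component and weapon reference are used without validity checks.
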(fn ReceivedNotifyEnd
  (params (MeshComp :type Skeletal%20Mesh%20Component%20Object%20Reference) (Animation :type Anim%20Sequence%20Base%20Object%20Reference) (EventReference :type Anim%20Notify%20Event%20Reference%20Structure%20%28by%20ref%29))
  (Default|DeactivateHitbox (Variables|/Game/Combat/Weapons/BPC_Weaponry.BPC_Weaponry_C|GetWeapon%20Ref (Actor|GetComponentbyClass (Components|GetOwner MeshComp) "/Game/Combat/Weapons/BPC_Weaponry.BPC_Weaponry_C")))
  (return false))

(fn ReceivedNotifyBegin
  (params (MeshComp :type Skeletal%20Mesh%20Component%20Object%20Reference) (Animation :type Anim%20Sequence%20Base%20Object%20Reference) (TotalDuration :type Float%20%28single-precision%29) (EventReference :type Anim%20Notify%20Event%20Reference%20Structure%20%28by%20ref%29))
  (Default|ActivateHitbox (Variables|/Game/Combat/Weapons/BPC_Weaponry.BPC_Weaponry_C|GetWeapon%20Ref (Actor|GetComponentbyClass (Components|GetOwner MeshComp) "/Game/Combat/Weapons/BPC_Weaponry.BPC_Weaponry_C")))
  (return false))