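; Anim notify state that clears the owner's melee attack state when its window in an animation ends.
; On notify end, a HeavyAttack flag selects whether to clear HeavyAttacking or Attacking on the owner's BPC_Melee component.
; It then sends the matching update message to the mesh's anim instance with false.
; Notify begin does nothing, so the notify only switches these states off.
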(fn ReceivedNotifyBegin
  (params (MeshComp :type Skeletal%20Mesh%20Component%20Object%20Reference) (Animation :type Anim%20Sequence%20Base%20Object%20Reference) (TotalDuration :type Float%20%28single-precision%29) (EventReference :type Anim%20Notify%20Event%20Reference%20Structure%20%28by%20ref%29))
  (return false))

(fn ReceivedNotifyEnd
  (params (MeshComp :type Skeletal%20Mesh%20Component%20Object%20Reference) (Animation :type Anim%20Sequence%20Base%20Object%20Reference) (EventReference :type Anim%20Notify%20Event%20Reference%20Structure%20%28by%20ref%29))
  (bind _returnvalue (Components|SkeletalMesh|GetAnimInstance MeshComp))
  (bind _returnvalue_2 (Components|GetOwner MeshComp))
  (bind _returnvalue_3 (Actor|GetComponentbyClass _returnvalue_2 "/Game/Combat/Melee/BPC_Melee.BPC_Melee_C"))
  (if (Variables|Default|GetHeavy%20Attack?)
    (Variables|/Game/Combat/Melee/BPC_Melee.BPC_Melee_C|SetHeavy%20Attacking _returnvalue_3 false)
    (Class|BPIPlayerAnimationBlueprint|UpdateHeavyAttacking(Message) _returnvalue false)
    (else
      (Variables|/Game/Combat/Melee/BPC_Melee.BPC_Melee_C|SetAttacking _returnvalue_3 false)
      (Class|BPIPlayerAnimationBlueprint|UpdateAttacking(Message) _returnvalue false)))
  (return false))