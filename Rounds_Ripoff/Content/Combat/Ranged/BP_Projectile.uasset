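; BP_Projectile is a reusable ranged-combat projectile that is activated and deactivated in place rather than spawned or destroyed.
; Both transitions route through server-to-multicast events that toggle visibility and the active flag, with collision disabled in both states.
; Activation applies speed, damage and mesh from a ProjectileInfo struct, launching along the actor's forward vector.
; An optional self-restarting timeline spins the mesh, while projectile stop only prints debug text.
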(event OnProjectileStop(ProjectileMovement)
  (params (ImpactResult :type Hit%20Result%20Structure%20%28by%20ref%29))
  (Development|PrintString "PROJECTILE STOP"))

(event Custom|%28multi%29%20Activate%20Projectile
  (params (Projectile%20Info :type Struct%20Projectile%20Info%20Structure))
  (Variables|Default|SetActive? true)
  (bind _output_get (Variables|Default|SetCurrent%20Projectile%20Info Projectile%20Info))
  (Rendering|SetActorHiddenInGame false)
  (Collision|SetActorEnableCollision false)
  (bind _output_get_2 (Variables|/Script/Engine.ProjectileMovementComponent|SetInitialSpeed (Variables|Default|GetProjectileMovement) (.Speed (Utilities|Struct|BreakStruct_Projectile_Info _output_get))))
  (bind _output_get_3 (Variables|/Script/Engine.ProjectileMovementComponent|SetMaxSpeed (Variables|Default|GetProjectileMovement) _output_get_2))
  (Variables|/Script/Engine.MovementComponent|SetVelocity (Variables|Default|GetProjectileMovement) (* _output_get_3 (Math|Vector|GetForwardVector (Transformation|GetActorRotation))))
  (Variables|Default|SetDamage (.Damage (Utilities|Struct|BreakStruct_Projectile_Info _output_get)))
  (Components|StaticMesh|SetStaticMesh (Variables|Default|GetProjectile%20Mesh) (.Mesh (Utilities|Struct|BreakStruct_Projectile_Info _output_get)))
  (Components|Movement|SetUpdatedComponent (Variables|Default|GetProjectileMovement) (Variables|Default|GetRoot))
  (if (Utilities|Struct|BreakStruct_Projectile_Info (Variables|Default|GetCurrent%20Projectile%20Info))
    (CallFunction|StartSpinProjectile)))

(event Custom|%28server%29%20Activate%20Projectile
  (params (Projectile%20Info :type Struct%20Projectile%20Info%20Structure))
  (CallFunction|(multi)ActivateProjectile Projectile%20Info))

(event Custom|%28server%29%20Deactivate%20Projectile
  (CallFunction|(multi)DeactivateProjectie))

(event Custom|%28multi%29%20Deactivate%20Projectie
  (Variables|Default|SetActive? false)
  (Rendering|SetActorHiddenInGame true)
  (Collision|SetActorEnableCollision false)
  (Transformation|SetActorLocationAndRotation "0, 0, 0" "0, 0, 0"))

(event Custom|Start%20Spin%20Projectile
  (Components|Timeline|SetPlayRate (Variables|Default|GetSpin%20Projectile%20Timeline) (/ 1.0 (Utilities|Struct|BreakStruct_Projectile_Info (Variables|Default|GetCurrent%20Projectile%20Info))))
  (CallFunction|SpinProjectileLoop))

(event Custom|Spin%20Projectile%20Loop
  (bind _alpha (Timeline|Spin%20Projectile%20Timeline PlayFromStart)
    (:Update
      (Transformation|SetRelativeRotation (Variables|Default|GetProjectile%20Mesh) (Math|Rotator|Lerp(Rotator) "0, 0, 0" "0.000000,360.000000,0.000000" _alpha) false false))
    (:Finished
      (if (Variables|Default|GetActive?)
        (CallFunction|SpinProjectileLoop)
        (else
          (CallFunction|StopProjectileSpin))))))

(event Custom|Stop%20Projectile%20Spin
  (bind _alpha (Timeline|Spin%20Projectile%20Timeline Stop)
    (:Update
      (Transformation|SetRelativeRotation (Variables|Default|GetProjectile%20Mesh) (Math|Rotator|Lerp(Rotator) "0, 0, 0" "0.000000,360.000000,0.000000" _alpha) false false))
    (:Finished
      (if (Variables|Default|GetActive?)
        (CallFunction|SpinProjectileLoop)
        (else
          (CallFunction|StopProjectileSpin))))))

(event EventActivateProjectile
  (params (Projectile%20Info :type Struct%20Projectile%20Info%20Structure))
  (CallFunction|(server)ActivateProjectile Projectile%20Info))

(event EventDeactivateProjectile
  (CallFunction|(server)DeactivateProjectile)
  (CallFunction|StopProjectileSpin))

(fn ConstructionScript)