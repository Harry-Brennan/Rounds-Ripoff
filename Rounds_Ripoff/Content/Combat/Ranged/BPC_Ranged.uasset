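; Ranged attack component that fires pooled BP_Projectile actors from its owner.
; On BeginPlay the authority spawns a hidden, collision-disabled pool and cycles through it round-robin without checking whether projectiles are in use.
; IA_Ranged input reaches a multicast, via server RPC from clients, setting Throwing for one second everywhere.
; Only the authority activates the next projectile just ahead of the owner, using its yaw and the current projectile info.
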(event Custom|%28multi%29%20Ranged%20Attack
  (bind _returnvalue (Components|GetOwner))
  (Variables|Default|SetThrowing true)
  (Networking|SwitchHasAuthority
    (:Authority
      (bind _projectile (Utilities|GetNextAvailableProjectile)
        (:Done
          (CallFunction|ActivateProjectile _projectile (+ (* (Transformation|GetActorForwardVector _returnvalue) 5e+01) (Transformation|GetActorLocation _returnvalue)) (Math|Rotator|MakeRotator 0.0 0.0 (.yaw (Transformation|GetActorRotation (Components|GetOwner))))))))
    (:Remote
      _))
  (Utilities|FlowControl|Delay 1.0)
  (Variables|Default|SetThrowing false))

(event Custom|%28server%29%20Ranged%20Attack
  (CallFunction|(multi)RangedAttack))

(event Custom|Spawn%20Projectile%20Pool
  (for _index (range 0 (- (Variables|Default|GetProjectile%20Pool%20Amount) 1))
    (bind _returnvalue (Game|SpawnActorfromClass "/Game/Combat/Ranged/BP_Projectile.BP_Projectile_C" (Math|Transform|MakeTransform "0, 0, 0" "0, 0, 0" "1.000000,1.000000,1.000000") "AlwaysSpawn" "MultiplyWithRoot" (Components|GetOwner) 0))
    (Rendering|SetActorHiddenInGame _returnvalue true)
    (Collision|SetActorEnableCollision _returnvalue false)
    (Utilities|Array|Add (Variables|Default|GetProjectile%20Pool) _returnvalue)))

(event Custom|Activate%20Projectile
  (params (Projectile :type BP%20Projectile%20Object%20Reference) (Activation%20Loc :type Vector) (Activation%20Rot :type Rotator))
  (Transformation|SetActorLocationAndRotation Projectile Activation%20Loc Activation%20Rot)
  (Default|ActivateProjectile Projectile (Variables|Default|GetCurrent%20Projectile%20Info)))

(event Custom|Deactivate%20Projectile
  (params (Projectile :type BP%20Projectile%20Object%20Reference))
  (Default|DeactivateProjectile Projectile))

(event Custom|Update%20Projectile%20Info
  (params (New%20Projectile%20Info :type Struct%20Projectile%20Info%20Structure))
  (Variables|Default|SetCurrent%20Projectile%20Info New%20Projectile%20Info))

(event Input|EnhancedActionEvents|EnhancedInputActionIA_Ranged
  (params (ActionValue :type Boolean) (ElapsedSeconds :type Float%20%28double-precision%29) (TriggeredSeconds :type Float%20%28double-precision%29) (InputAction :type Input%20Action%20Object%20Reference :default "/Game/Input/Actions/In-Game/IA_Ranged.IA_Ranged"))
  (Development|PrintString "RANGED")
  (Networking|SwitchHasAuthority
    (:Authority
      (CallFunction|(multi)RangedAttack))
    (:Remote
      (CallFunction|(server)RangedAttack))))

(event EventBeginPlay
  (Networking|SwitchHasAuthority
    (:Authority
      (CallFunction|SpawnProjectilePool))))