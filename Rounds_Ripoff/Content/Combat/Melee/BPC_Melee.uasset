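; Melee combat component that handles normal attack and deflect input for its owner, with debug prints on the attack path.
; Input is gated by CanAttack and routed to the authority directly or through server RPCs.
; Deflect start and both stop events multicast their state, while attack start runs only on the authority.
; Attacking and Deflecting flags are pushed to the owner's skeletal mesh AnimInstance through message calls.
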(event Custom|%28server%29%20Deflect
  ;[0 0 0] Normal, and deflecting functionality
  (CallFunction|(multi)Deflect))

(event Custom|%28multi%29%20Deflect
  ;[0 0 0] Normal, and deflecting functionality
  (Variables|Default|SetDeflecting true)
  (Utilities|UpdateDeflectingAnim))

(event Custom|%28server%29%20Stop%20Normal%20Melee
  ;[0 0 0] Normal, and deflecting functionality
  (CallFunction|(multi)StopNormalMelee))

(event Custom|%28multi%29%20Stop%20Normal%20Melee
  ;[0 0 0] Normal, and deflecting functionality
  (Variables|Default|SetAttacking false)
  (Utilities|UpdateAttackingAnim))

(event Custom|%28server%29%20Stop%20Deflecting
  ;[0 0 0] Normal, and deflecting functionality
  (CallFunction|(multi)StopDeflecting))

(event Custom|%28multi%29%20Stop%20Deflecting
  ;[0 0 0] Normal, and deflecting functionality
  (Variables|Default|SetDeflecting false)
  (Utilities|UpdateDeflectingAnim))

(event Custom|%28server%29%20Normal%20Melee
  ;[0 0 0] Normal, and deflecting functionality
  (CallFunction|MeleeNormal)
  (Development|PrintString "NORMAL MELEE SERVER"))

(event Custom|Melee%20Normal
  ;[0 0 0] Normal, and deflecting functionality
  (Development|PrintString "NORMAL MELEE CLIENT")
  (Variables|Default|SetAttacking true)
  (Utilities|UpdateAttackingAnim))

(event Input|EnhancedActionEvents|EnhancedInputActionIA_Deflect
  (params (ActionValue :type Boolean) (ElapsedSeconds :type Float%20%28double-precision%29) (TriggeredSeconds :type Float%20%28double-precision%29) (InputAction :type Input%20Action%20Object%20Reference :default "/Game/Input/Actions/IA_Deflect.IA_Deflect"))
  ;[0 0 0] Normal, and deflecting input actions
  (if (Utilities|CanAttack)
    (Networking|SwitchHasAuthority
      (:Authority
        (CallFunction|(multi)Deflect))
      (:Remote
        (CallFunction|(server)Deflect)))))

(event Input|EnhancedActionEvents|EnhancedInputActionIA_Melee
  (params (ActionValue :type Boolean) (ElapsedSeconds :type Float%20%28double-precision%29) (TriggeredSeconds :type Float%20%28double-precision%29) (InputAction :type Input%20Action%20Object%20Reference :default "/Game/Input/Actions/IA_Melee.IA_Melee"))
  ;[0 0 0] Normal, and deflecting input actions
  (if (Utilities|CanAttack)
    (Development|PrintString "NORMAL ATTACK")
    (Networking|SwitchHasAuthority
      (:Authority
        (CallFunction|MeleeNormal))
      (:Remote
        (CallFunction|(server)NormalMelee)))
    (else
      (Development|PrintString "CAN ATTACK FALSE"))))