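; Base melee weapon Blueprint that provides a toggleable hitbox for dealing damage and knockback.
; While active, a looping timer box-traces pawns and physics bodies at the mesh's Hitbox socket, ignoring the owner.
; A per-actor timestamp map enforces a short re-hit cooldown.
; Targets with BPC_Health receive server damage and knockback away from the owner, amplified for BPI_Hazard actors; others get an impact-based force.
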(event Custom|Hitbox%20Loop
  (bind _knockback_amount (Variables|Default|GetKnockback%20Amount))
  (bind _weapon_mesh (Variables|Default|GetWeapon%20Mesh))
  (bind _returnvalue (Transformation|GetSocketLocation _weapon_mesh "Hitbox"))
  (bind _outhits (Class|KismetSystemLibrary|BoxTraceMultiforObjects _returnvalue _returnvalue (Variables|Default|GetHitbox%20Size) (Transformation|GetSocketRotation (Variables|Default|GetWeapon%20Mesh) "Hitbox") (Utilities|Array|MakeArray "ObjectTypeQuery3" "ObjectTypeQuery4") false (Utilities|Array|MakeArray (Components|GetOwner)) "ForOneFrame" true))
  (for _array_element _outhits
    (if (.ReturnValue (Utilities|Map|Find (Variables|Default|GetHit%20Actor%20-%20Time) (.HitActor (Collision|BreakHitResult _array_element))))
      (if (>= (- (Utilities|Time|GetGameTimeinSeconds) (.Value (Utilities|Map|Find (Variables|Default|GetHit%20Actor%20-%20Time) (.HitActor (Collision|BreakHitResult _array_element))))) 0.25)
        (Utilities|Map|Add (Variables|Default|GetHit%20Actor%20-%20Time) (.HitActor (Collision|BreakHitResult _array_element)) (Utilities|Time|GetGameTimeinSeconds) :!label _label)
        (Utilities|IsValid (Actor|GetComponentbyClass (.HitActor (Collision|BreakHitResult _array_element)) "/Game/Health/BPC_Health.BPC_Health_C")
          (:Is%20Valid
            (Default|(server)TakeDamage (Actor|GetComponentbyClass (.HitActor (Collision|BreakHitResult _array_element)) "/Game/Health/BPC_Health.BPC_Health_C") (Variables|Default|GetDamage) (.Location (Collision|BreakHitResult _array_element)))
            (Default|(server)Knockback (Actor|GetComponentbyClass (.HitActor (Collision|BreakHitResult _array_element)) "/Game/Health/BPC_Health.BPC_Health_C") (Math|Vector|MakeVector (.x (* (- (Transformation|GetActorLocation (Components|GetOwner)) (Transformation|GetActorLocation (.HitActor (Collision|BreakHitResult _array_element)))) -1.0)) (.y (* (- (Transformation|GetActorLocation (Components|GetOwner)) (Transformation|GetActorLocation (.HitActor (Collision|BreakHitResult _array_element)))) -1.0)) 25.0) (Math|Float|SelectFloat (* _knockback_amount 5.0) _knockback_amount (Utilities|DoesObjectImplementInterface (.HitActor (Collision|BreakHitResult _array_element)) "/Game/Hazards/BPI_Hazard.BPI_Hazard_C"))))
          (:Is%20Not%20Valid
            (Physics|AddForce (.HitComponent (Collision|BreakHitResult _array_element)) (Math|Vector|MakeVector (.x (* (* (.ImpactNormal (Collision|BreakHitResult _array_element)) (* (Variables|Default|GetKnockback%20Amount) 75.0)) -1.0)) (.y (* (* (.ImpactNormal (Collision|BreakHitResult _array_element)) (* (Variables|Default|GetKnockback%20Amount) 75.0)) -1.0)) 2.5e+02) "None" true))))
      (else
        (goto _label)))))

(event EventDeactivateHitbox
  (Utilities|Time|ClearandInvalidateTimerbyHandle (Variables|Default|GetHitbox%20Loop%20Timer)))

(event EventActivateHitbox
  (bind _returnvalue (Utilities|Time|SetTimerbyEvent (delegate Custom|Hitbox%20Loop) (Variables|Default|GetHitbox%20Tick) true))
  (Variables|Default|SetHitbox%20Loop%20Timer _returnvalue))

(fn ConstructionScript)