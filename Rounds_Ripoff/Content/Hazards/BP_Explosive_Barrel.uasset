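; Explosive barrel hazard that damages itself on hard impacts and triggers a server explosion through BPCExplode at its location when destroyed.
; A velocity detection mesh caches the barrel's velocity and game time on overlap, capturing speed before the collision.
; When the main mesh hits another actor shortly afterward at sufficient cached speed, BPCHealth takes server damage proportional to that speed.
; The overlap event also prints debug strings.
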(event OnComponentBeginOverlap(VelocityDetectionMesh)
  (params (OverlappedComponent :type Primitive%20Component%20Object%20Reference) (OtherActor :type Actor%20Object%20Reference) (OtherComp :type Primitive%20Component%20Object%20Reference) (OtherBodyIndex :type Integer) (bFromSweep :type Boolean) (SweepResult :type Hit%20Result%20Structure%20%28by%20ref%29))
  (bind _main_hazard_mesh (Variables|Default|GetMain%20Hazard%20Mesh))
  (bind _returnvalue (Transformation|GetComponentVelocity _main_hazard_mesh))
  (Development|PrintString "BARREL VELOCITY DETECTION")
  (Utilities|Map|Clear (Variables|Default|GetVelocity%20Before%20Hit%20-%20Time%20of%20Hit))
  (Utilities|Map|Add (Variables|Default|GetVelocity%20Before%20Hit%20-%20Time%20of%20Hit) _returnvalue (Utilities|Time|GetGameTimeinSeconds))
  (Development|PrintString (Utilities|String|ToString(Float) (Math|Vector|VectorLength _returnvalue))))

(event OnComponentHit(MainHazardMesh)
  (params (HitComponent :type Primitive%20Component%20Object%20Reference) (OtherActor :type Actor%20Object%20Reference) (OtherComp :type Primitive%20Component%20Object%20Reference) (NormalImpulse :type Vector :default "0, 0, 0") (Hit :type Hit%20Result%20Structure%20%28by%20ref%29))
  (bind _velocity_before_hit___time_of_hit (Variables|Default|GetVelocity%20Before%20Hit%20-%20Time%20of%20Hit))
  (if (not (== OtherActor self))
    (bind _keys (Utilities|Map|Keys _velocity_before_hit___time_of_hit))
    (bind _values (Utilities|Map|Values _velocity_before_hit___time_of_hit))
    (if (>= (Math|Vector|VectorLength (Utilities|Array|Get(acopy) _keys)) (Variables|Default|GetMin%20Velocity%20For%20Damage))
      (if (<= (- (Utilities|Time|GetGameTimeinSeconds) (Utilities|Array|Get(acopy) _values)) 0.25)
        (Default|(server)TakeDamage (Variables|Default|GetBPC_Health) (/ (Math|Vector|VectorLength (Utilities|Array|Get(acopy) _keys)) 4.0) (Transformation|GetActorLocation))))))

(event EventBeginPlay
  (|CallParentFunction))

(event EventHazardDeath/Destruction
  (Default|(server)Explode (Variables|Default|GetBPC_Explode) (Transformation|GetActorLocation)))

(fn ConstructionScript
  (|CallParentFunction))