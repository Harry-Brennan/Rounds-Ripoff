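; Actor component that makes its owner explode, with server events for the blast and its effects.
; A sphere trace at the epicentre hits each pawn or physics actor once, scaling by distance from the centre.
; BPC_Health owners take damage and knockback, while other hit components get an impulse-like AddForce.
; A multicast hides the owner, disables its collision, and plays particles, camera shake and sound.
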(event Custom|%28server%29%20Explode
  (params (Explosion%20Epicentre :type Vector))
  (CallFunction|Explode Explosion%20Epicentre))

(event Custom|Explode
  (params (Explosion%20Epicentre :type Vector))
  (Utilities|Array|Clear (Variables|Default|GetHit%20Actors))
  (bind _output_get (Variables|Default|SetExplosion%20Epicentre Explosion%20Epicentre))
  (CallFunction|(server)ExplodeCosmetic _output_get (Variables|Default|GetExplosion%20Emitter?) (Variables|Default|GetExplosion%20SFX%20Emitter) (Variables|Default|GetExplosion%20SFX%20Niagara))
  (bind _outhits (Collision|MultiSphereTraceForObjects _output_get _output_get (Variables|Default|GetExplosion%20Radius) (Utilities|Array|MakeArray "ObjectTypeQuery4" "ObjectTypeQuery3") false (Utilities|Array|MakeArray (Components|GetOwner)) "ForDuration"))
  (for _array_element _outhits
    (if (not (Utilities|Array|ContainsItem (Variables|Default|GetHit%20Actors) (.HitActor (Collision|BreakHitResult _array_element))))
      (Utilities|Array|Add (Variables|Default|GetHit%20Actors) (.HitActor (Collision|BreakHitResult _array_element)))
      (Utilities|IsValid (Actor|GetComponentbyClass (.HitActor (Collision|BreakHitResult _array_element)) "/Game/Health/BPC_Health.BPC_Health_C")
        (:Is%20Valid
          (Default|(server)TakeDamage (Actor|GetComponentbyClass (.HitActor (Collision|BreakHitResult _array_element)) "/Game/Health/BPC_Health.BPC_Health_C") (* (Variables|Default|GetExplosion%20Max%20Damage) (- 1.0 (/ (Math|Vector|VectorLength (- (Variables|Default|GetExplosion%20Epicentre) (.Location (Collision|BreakHitResult _array_element)))) (Variables|Default|GetExplosion%20Radius)))) (.Location (Collision|BreakHitResult _array_element)))
          (Default|(server)Knockback (Actor|GetComponentbyClass (.HitActor (Collision|BreakHitResult _array_element)) "/Game/Health/BPC_Health.BPC_Health_C") (* (.ImpactNormal (Collision|BreakHitResult _array_element)) -1.0) (* (- 1.0 (/ (Math|Vector|VectorLength (- (Variables|Default|GetExplosion%20Epicentre) (.Location (Collision|BreakHitResult _array_element)))) (Variables|Default|GetExplosion%20Radius))) (Variables|Default|GetExplosion%20Max%20Knockback))))
        (:Is%20Not%20Valid
          (Physics|AddForce (.HitComponent (Collision|BreakHitResult _array_element)) (* (* (.ImpactNormal (Collision|BreakHitResult _array_element)) -1.0) (* (* (- 1.0 (/ (Math|Vector|VectorLength (- (Variables|Default|GetExplosion%20Epicentre) (.Location (Collision|BreakHitResult _array_element)))) (Variables|Default|GetExplosion%20Radius))) (Variables|Default|GetExplosion%20Max%20Knockback)) 5.0)) "None" true))))))

(event Custom|%28multi%29%20Explode%20Cosmetic
  (params (Explosion%20Location :type Vector) (Emitter? :type Boolean) (Emitter :type Particle%20System%20Object%20Reference) (Niagara :type Niagara%20System%20Object%20Reference))
  (bind _returnvalue (Components|GetOwner))
  (Development|PrintString "EXPLODE COSTMETIC" true true "(R=0.000000,G=0.660000,B=1.000000,A=1.000000)" 1e+02)
  (Rendering|SetActorHiddenInGame _returnvalue true)
  (Collision|SetActorEnableCollision _returnvalue false)
  (if Emitter?
    (Effects|SpawnEmitteratLocation Emitter Explosion%20Location "0, 0, 0" "5.000000,5.000000,5.000000")
    (else
      (Niagara|SpawnSystematLocation Niagara Explosion%20Location)))
  (Class|LegacyCameraShake|StartLegacyCameraShake (Game|GetPlayerCameraManager 0) "/Game/Hazards/BP_Explosion_Camera_Shake.BP_Explosion_Camera_Shake_C" 0.5 "CameraLocal" "0, 0, 0")
  (Audio|PlaySoundatLocation "/Game/StarterContent/Audio/Explosion_Cue.Explosion_Cue" Explosion%20Location "0, 0, 0" 1.0 1.0 0.0 0 0 0 0))

(event Custom|%28server%29%20Explode%20Cosmetic
  (params (Explosion%20Location :type Vector) (Emitter? :type Boolean) (E,mitter :type Particle%20System%20Object%20Reference) (Niagara :type Niagara%20System%20Object%20Reference))
  (CallFunction|(multi)ExplodeCosmetic Explosion%20Location Emitter? E,mitter Niagara))

(fn OnRepExplosionEpicentre)