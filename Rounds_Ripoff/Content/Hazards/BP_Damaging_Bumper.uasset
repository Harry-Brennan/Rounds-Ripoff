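; Damaging bumper hazard that hurts and knocks back overlapping actors that have a health component.
; On PlayerDetectionCollision overlap, it looks up BPC_Health and calls ServerTakeDamage with its Damage value and location.
; It then calls ServerKnockback along the unnormalized horizontal offset away from the bumper, with a fixed upward component and KnockbackAmount strength.
; Actors without the component only trigger a debug print.
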(event OnComponentBeginOverlap(PlayerDetectionCollision)
  (params (OverlappedComponent :type Primitive%20Component%20Object%20Reference) (OtherActor :type Actor%20Object%20Reference) (OtherComp :type Primitive%20Component%20Object%20Reference) (OtherBodyIndex :type Integer) (bFromSweep :type Boolean) (SweepResult :type Hit%20Result%20Structure%20%28by%20ref%29))
  (bind _returnvalue (Actor|GetComponentbyClass OtherActor "/Game/Health/BPC_Health.BPC_Health_C"))
  (bind _returnvalue_2 (Transformation|GetActorLocation OtherActor))
  (bind _returnvalue_3 (Transformation|GetActorLocation))
  (bind _returnvalue_4 (- _returnvalue_2 _returnvalue_3))
  (Utilities|IsValid _returnvalue
    (:Is%20Valid
      (Default|(server)TakeDamage _returnvalue (Variables|Default|GetDamage) _returnvalue_3)
      (Default|(server)Knockback _returnvalue (Math|Vector|MakeVector (.x _returnvalue_4) (.y _returnvalue_4) 15.0) (Variables|Default|GetKnockback%20Amount)))
    (:Is%20Not%20Valid
      (Development|PrintString "HEALTH COMPONENT NOT VALID"))))

(event EventBeginPlay
  (|CallParentFunction) ; This node is disabled and will not be called.\nDrag off pins to build functionality.
)

(fn ConstructionScript
  (|CallParentFunction))