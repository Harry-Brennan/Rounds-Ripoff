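; Rotating saw hazard that damages players, starts on BeginPlay and can be stopped.
; A looping timer spins two blades while a restarting timeline moves each along its own spline, keeping the damage volume at their midpoint.
; An overlap enables Tick, which damages overlapping players through BPC_Health and switches itself off once none remain.
; A per-actor timestamp map limits hits to one per quarter second.
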(event OnComponentBeginOverlap(DamageHitDetection)
  (params (OverlappedComponent :type Primitive%20Component%20Object%20Reference) (OtherActor :type Actor%20Object%20Reference) (OtherComp :type Primitive%20Component%20Object%20Reference) (OtherBodyIndex :type Integer) (bFromSweep :type Boolean) (SweepResult :type Hit%20Result%20Structure%20%28by%20ref%29))
  (Actor|Tick|SetActorTickEnabled true))

(event Custom|Rotate%20Saw%20Blade
  (Transformation|AddRelativeRotation (Variables|Default|GetSaw%20Blade) (Math|Rotator|MakeRotator 5.0 0.0 0.0) false false))

(event Custom|Loop%20Saw%20Movement
  (bind _saw_blade_2_spline (Variables|Default|GetSaw%20Blade%202%20Spline))
  (bind _saw_blade_spline (Variables|Default|GetSaw%20Blade%20Spline))
  (bind _alpha (Timeline|Move%20Saw%20Blade%20Timeline PlayFromStart)
    (:Update
      (Transformation|SetWorldLocation (Variables|Default|GetSaw%20Blade) (Spline|GetLocationatDistanceAlongSpline _saw_blade_spline (* (Spline|GetSplineLength _saw_blade_spline) _alpha) "World") false false)
      (Transformation|SetWorldLocation (Variables|Default|GetSaw%20Blade%202) (Spline|GetLocationatDistanceAlongSpline _saw_blade_2_spline (* (Spline|GetSplineLength _saw_blade_2_spline) _alpha) "World") false false)
      (Transformation|SetWorldLocation (Variables|Default|GetDamage%20Hit%20Detection) (+ (/ (- (Transformation|GetWorldLocation (Variables|Default|GetSaw%20Blade%202)) (Transformation|GetWorldLocation (Variables|Default|GetSaw%20Blade))) 2.0) (Transformation|GetWorldLocation (Variables|Default|GetSaw%20Blade))) false false))
    (:Finished
      (if (Variables|Default|GetActive?)
        (CallFunction|LoopSawMovement)))))

(event EventBeginPlay
  (|CallParentFunction)
  (CallFunction|StartHazard))

(event EventStartHazard
  (bind _saw_blade_2_spline (Variables|Default|GetSaw%20Blade%202%20Spline))
  (bind _saw_blade_spline (Variables|Default|GetSaw%20Blade%20Spline))
  (Variables|Default|SetActive? true)
  (Utilities|FlowControl|Sequence
    (:then_0
      (bind _returnvalue (Utilities|Time|SetTimerbyEvent (delegate Custom|Rotate%20Saw%20Blade) (Variables|Default|GetSaw%20Blade%20Rotate%20Speed) true))
      (Variables|Default|SetRotate%20Timer _returnvalue)
      (Components|Timeline|SetPlayRate (Variables|Default|GetMove%20Saw%20Blade%20Timeline) (/ 1.0 (Variables|Default|GetSaw%20Blade%20Move%20Speed))))
    (:then_1
      (bind _alpha (Timeline|Move%20Saw%20Blade%20Timeline Play)
        (:Update
          (Transformation|SetWorldLocation (Variables|Default|GetSaw%20Blade) (Spline|GetLocationatDistanceAlongSpline _saw_blade_spline (* (Spline|GetSplineLength _saw_blade_spline) _alpha) "World") false false)
          (Transformation|SetWorldLocation (Variables|Default|GetSaw%20Blade%202) (Spline|GetLocationatDistanceAlongSpline _saw_blade_2_spline (* (Spline|GetSplineLength _saw_blade_2_spline) _alpha) "World") false false)
          (Transformation|SetWorldLocation (Variables|Default|GetDamage%20Hit%20Detection) (+ (/ (- (Transformation|GetWorldLocation (Variables|Default|GetSaw%20Blade%202)) (Transformation|GetWorldLocation (Variables|Default|GetSaw%20Blade))) 2.0) (Transformation|GetWorldLocation (Variables|Default|GetSaw%20Blade))) false false))
        (:Finished
          (if (Variables|Default|GetActive?)
            (CallFunction|LoopSawMovement)))))
    (:then_2
      (Variables|/Script/Engine.PrimitiveComponent|SetbGenerateOverlapEvents (Variables|Default|GetDamage%20Hit%20Detection) true))))

(event EventStopHazard
  (bind _saw_blade_2_spline (Variables|Default|GetSaw%20Blade%202%20Spline))
  (bind _saw_blade_spline (Variables|Default|GetSaw%20Blade%20Spline))
  (Variables|Default|SetActive? false)
  (Utilities|FlowControl|Sequence
    (:then_0
      (bind _alpha (Timeline|Move%20Saw%20Blade%20Timeline Stop)
        (:Update
          (Transformation|SetWorldLocation (Variables|Default|GetSaw%20Blade) (Spline|GetLocationatDistanceAlongSpline _saw_blade_spline (* (Spline|GetSplineLength _saw_blade_spline) _alpha) "World") false false)
          (Transformation|SetWorldLocation (Variables|Default|GetSaw%20Blade%202) (Spline|GetLocationatDistanceAlongSpline _saw_blade_2_spline (* (Spline|GetSplineLength _saw_blade_2_spline) _alpha) "World") false false)
          (Transformation|SetWorldLocation (Variables|Default|GetDamage%20Hit%20Detection) (+ (/ (- (Transformation|GetWorldLocation (Variables|Default|GetSaw%20Blade%202)) (Transformation|GetWorldLocation (Variables|Default|GetSaw%20Blade))) 2.0) (Transformation|GetWorldLocation (Variables|Default|GetSaw%20Blade))) false false))
        (:Finished
          (if (Variables|Default|GetActive?)
            (CallFunction|LoopSawMovement)))))
    (:then_1
      (Utilities|Time|ClearandInvalidateTimerbyHandle (Variables|Default|GetRotate%20Timer)))
    (:then_2
      (Variables|/Script/Engine.PrimitiveComponent|SetbGenerateOverlapEvents (Variables|Default|GetDamage%20Hit%20Detection) false))))

(event EventTick
  (params (DeltaSeconds :type Float%20%28single-precision%29))
  (bind _damage_hit_detection (Variables|Default|GetDamage%20Hit%20Detection))
  (bind _overlappingactors (Collision|GetOverlappingActors _damage_hit_detection "/Game/Player/BP_Player.BP_Player_C" :!class /Script/Engine.PrimitiveComponent))
  (if (Utilities|Array|IsEmpty _overlappingactors)
    (Actor|Tick|SetActorTickEnabled false)
    (else
      (for _array_element _overlappingactors
        (CallFunction|SawBladeDamage _array_element)))))

(fn ConstructionScript
  (|CallParentFunction))

(fn SawBladeDamage
  (params (Hit%20Actor :type Actor%20Object%20Reference%20%28by%20ref%29))
  (bind _returnvalue (Actor|GetComponentbyClass Hit%20Actor "/Game/Health/BPC_Health.BPC_Health_C"))
  (bind _returnvalue_2 (Utilities|Time|GetGameTimeinSeconds))
  (bind _hit_actors___time (Variables|Default|GetHit%20Actors%20-%20Time))
  (bind (_value _returnvalue_3) (Utilities|Map|Find _hit_actors___time Hit%20Actor))
  (Utilities|IsValid _returnvalue
    (:Is%20Valid
      (if _returnvalue_3
        (if (>= (- (Utilities|Time|GetGameTimeinSeconds) _value) 0.25)
          (Utilities|Map|Add (Variables|Default|GetHit%20Actors%20-%20Time) Hit%20Actor _returnvalue_2 :!label _label)
          (Development|PrintString (Utilities|String|Append "SAW BLADE DAMAGE : " (Utilities|String|ToString(Float) _returnvalue_2)))
          (Default|(server)TakeDamage _returnvalue (Variables|Default|GetDamage) (Transformation|GetActorLocation)))
        (else
          (goto _label))))))