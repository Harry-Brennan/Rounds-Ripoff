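; BP_Spikes is a spike hazard that damages actors with a health component when they hit its main hazard mesh.
; On each hit it calls ServerTakeDamage on the actor's BPC_Health, passing the damage amount and the spikes' location.
; A map of last-hit times per actor limits damage to once per second for each victim, with a debug print on every damaging hit.
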(event OnComponentHit(MainHazardMesh)
  (params (HitComponent :type Primitive%20Component%20Object%20Reference) (OtherActor :type Actor%20Object%20Reference) (OtherComp :type Primitive%20Component%20Object%20Reference) (NormalImpulse :type Vector :default "0, 0, 0") (Hit :type Hit%20Result%20Structure%20%28by%20ref%29))
  (bind _returnvalue (Actor|GetComponentbyClass OtherActor "/Game/Health/BPC_Health.BPC_Health_C"))
  (bind _hit_players___time_hit (Variables|Default|GetHit%20Players%20-%20Time%20Hit))
  (bind (_value _returnvalue_2) (Utilities|Map|Find _hit_players___time_hit OtherActor))
  (Utilities|IsValid _returnvalue
    (:Is%20Valid
      (if _returnvalue_2
        (if (>= (- (Utilities|Time|GetGameTimeinSeconds) _value) 1.0)
          (Utilities|Map|Add (Variables|Default|GetHit%20Players%20-%20Time%20Hit) OtherActor (Utilities|Time|GetGameTimeinSeconds) :!label _label)
          (Development|PrintString "SPIKE TAKE DAMAGE")
          (Default|(server)TakeDamage _returnvalue (Variables|Default|GetDamage) (Transformation|GetActorLocation)))
        (else
          (goto _label))))))

(event EventBeginPlay
  (|CallParentFunction) ; This node is disabled and will not be called.\nDrag off pins to build functionality.
)

(fn ConstructionScript
  (|CallParentFunction))