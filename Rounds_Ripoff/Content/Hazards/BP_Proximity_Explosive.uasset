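; BP_Proximity_Explosive is a hazard that explodes a set time after something enters its detection collision.
; The first overlap starts a one-shot timer, which then deals lethal damage to its own health component.
; The death/destruction event calls the explode component's server explode at the actor's location, keeping detonation on the damage path.
; ResetHazard rearms the trigger and cancels any pending timer.
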(event OnComponentBeginOverlap(DetectionCollision)
  (params (OverlappedComponent :type Primitive%20Component%20Object%20Reference) (OtherActor :type Actor%20Object%20Reference) (OtherComp :type Primitive%20Component%20Object%20Reference) (OtherBodyIndex :type Integer) (bFromSweep :type Boolean) (SweepResult :type Hit%20Result%20Structure%20%28by%20ref%29))
  (Utilities|FlowControl|DoOnce false
    (:Completed
      (bind _returnvalue (Utilities|Time|SetTimerbyEvent (delegate Custom|Explode%20Timer) (Variables|Default|GetExplosion%20Time))))))

(event Custom|Explode%20Timer
  (Default|(server)TakeDamage (Variables|Default|GetBPC_Health) 999.0 (Transformation|GetActorLocation)))

(event EventBeginPlay
  (|CallParentFunction) ; This node is disabled and will not be called.\nDrag off pins to build functionality.
)

(event EventHazardDeath/Destruction
  (Default|(server)Explode (Variables|Default|GetBPC_Explode) (Transformation|GetActorLocation)))

(event EventResetHazard
  (Utilities|FlowControl|Sequence
    (:then_0
      (Utilities|FlowControl|DoOnce false) ; enters at Reset
    )
    (:then_1
      (Utilities|Time|ClearandInvalidateTimerbyHandle (stale OnComponentBeginOverlap(DetectionCollision) _returnvalue)))))

(fn ConstructionScript
  (|CallParentFunction))